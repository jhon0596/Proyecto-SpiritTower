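; AI controller for a patrolling pawn that follows a four-point route through a behavior tree.
; On BeginPlay it sets up the Patrullar blackboard, storing the pawn's starting location as the first position and three hardcoded world points as the others.
; It then runs the AC_Patrullar behavior tree, which receives those positions through the blackboard keys.
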(event EventBeginPlay
  (bind _blackboardcomponent (Class|AIController|UseBlackboard "/Game/Blueprints/AI/Blackboard_Patrullar.Blackboard_Patrullar"))
  (AI|Components|Blackboard|SetValueasVector _blackboardcomponent (Utilities|Name|MakeLiteralName "Posicion1") (Transformation|GetActorLocation (Pawn|GetControlledPawn)))
  (AI|Components|Blackboard|SetValueasVector _blackboardcomponent (Utilities|Name|MakeLiteralName "Posicion2") "-1100.000000,-1360.000000, 0")
  (AI|Components|Blackboard|SetValueasVector _blackboardcomponent (Utilities|Name|MakeLiteralName "Posicion3") "-1100.000000,240.000000, 0")
  (AI|Components|Blackboard|SetValueasVector _blackboardcomponent (Utilities|Name|MakeLiteralName "Posicion4") "430.000000,240.000000, 0")
  (AI|RunBehaviorTree "/Game/Blueprints/AI/AC_Patrullar.AC_Patrullar"))

(event EventTick
  (params (DeltaSeconds :type Float%20%28single-precision%29)))

(fn ConstructionScript)