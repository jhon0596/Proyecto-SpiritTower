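; Behavior tree decorator that checks whether the player is within vision range of an AI pawn run by Seguir_AIController.
; PerformConditionCheck casts the owner to that controller and passes when the straight-line distance from its pawn to player pawn 0 is at most RangodeVision.
; It prints the distance on each check for debugging.
; The EventGraph holds only a disconnected copy of the same logic.
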(fn PerformConditionCheck
  (params (OwnerActor :type Actor%20Object%20Reference))
  (bind _asseguir_aicontroller (Utilities|Casting|CastToSeguir_AIController OwnerActor))
  (Development|PrintString (Utilities|String|ToString(Float) (Math|Vector|VectorLength (- (Transformation|GetActorLocation (Pawn|GetControlledPawn _asseguir_aicontroller)) (Transformation|GetActorLocation (Game|Player|GetPlayerPawn 0))))))
  (return (<= (Math|Vector|VectorLength (- (Transformation|GetActorLocation (Pawn|GetControlledPawn _asseguir_aicontroller)) (Transformation|GetActorLocation (Game|Player|GetPlayerPawn 0)))) (Variables|Default|GetRangodeVision))))